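; BPCustomPlayerCharacter is a first-person player character that shoots projectiles from a gun held by its arms.
; The Fire input plays a firing montage on the Arms and calls SpawnProjectile from just below the camera location, aimed along the camera's forward vector.
; The construction script snaps the Gun to the GripPoint socket on the Arms.
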(event EventBeginPlay)

(event Input|ActionEvents|InputActionFire
  (params (Key :type Key%20Structure))
  (bind _firstpersoncamera (Variables|Default|GetFirstPersonCamera))
  (:Pressed
    (Animation|Montage|MontagePlay (Components|SkeletalMesh|GetAnimInstance (Variables|Default|GetArms)) "/Game/FirstPerson/Animations/FirstPersonFire_Montage.FirstPersonFire_Montage" 1.0 "MontageLength" 0.0 true)
    (Class|CustomPlayerCharacter|SpawnProjectile (- (Transformation|GetWorldLocation _firstpersoncamera) "0,0.000000,2.000000") (Math|Vector|GetForwardVector _firstpersoncamera))))

(fn ConstructionScript
  (Transformation|AttachComponentToComponent (Variables|Default|GetGun) (Variables|Default|GetArms) "GripPoint" "SnapToTarget" "SnapToTarget" "SnapToTarget" true))